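; BP_FocusCube is an interactable cube, apparently for testing, that highlights on focus and prints a message on a successful or failed interaction.
; The construction script creates a dynamic instance of M_FocusCube and applies it to the cube mesh.
; Focus changes drive that instance's color and emissive parameters, switching between glowing green and unlit grey.
; CanInteractWith returns the CanBeInteractedWith flag, ignoring the interactor's ability system component.
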(event `self.OnFocusChanged`
  (params (bIsFocus :type Boolean) (InteractorASC :type "AbilitySystemComponent Object Reference"))
  (bind _dynamicmaterial (`self.DynamicMaterial`))
  (bind _dynamicmaterial_2 (`self.DynamicMaterial`))
  (if bIsFocus
    (`MaterialInstanceDynamic.SetScalarParameterValue` _dynamicmaterial "EmisiveMultiplier" 1.0)
    (`MaterialInstanceDynamic.SetVectorParameterValue` _dynamicmaterial_2 "Color" (struct :`R` 0.279888 :`G` 0.6875 :`B` 0.255135 :`A` 1.0))
    (else
      (`MaterialInstanceDynamic.SetScalarParameterValue` _dynamicmaterial "EmisiveMultiplier" 0.0)
      (`MaterialInstanceDynamic.SetVectorParameterValue` _dynamicmaterial_2 "Color" (struct :`R` 0.802083 :`G` 0.802083 :`B` 0.802083 :`A` 1.0)))))

(event `self.Interact`
  (params (InteractorASC :type "AbilitySystemComponent Object Reference"))
  (`KismetSystemLibrary.PrintString` "I GOT IT!!"))

(event `self.InteractionFailed`
  (params (InteractorASC :type "AbilitySystemComponent Object Reference"))
  (`KismetSystemLibrary.PrintString` "failed"))

(fn `CanInteractWith`
  (params (InteractorASC :type "AbilitySystemComponent Object Reference"))
  (returns (ReturnValue :type Boolean))
  (return (`self.Can Be Interacted With?`)))

(fn `UserConstructionScript`
  (bind _returnvalue (`KismetMaterialLibrary.CreateDynamicMaterialInstance` "/Game/Interactables/M_FocusCube.M_FocusCube"))
  (bind _output_get (set `self.DynamicMaterial` _returnvalue))
  (`PrimitiveComponent.SetMaterial` (`self.Cube`) 0 _output_get))